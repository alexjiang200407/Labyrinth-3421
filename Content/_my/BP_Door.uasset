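; BP_Door is a hinged door that swings open when the first-person character walks into its trigger.
; On overlap it compares the door's yaw to the frame's and only proceeds when the two differ by less than five degrees, so an open door stays put.
; A timeline curve then lerps the door's relative yaw in the negative direction to its open angle, with no closing logic.
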(event `self.trigger.OnComponentBeginOverlap`
  (params (OverlappedComponent :type "PrimitiveComponent Object Reference") (OtherActor :type "Actor Object Reference") (OtherComp :type "PrimitiveComponent Object Reference") (OtherBodyIndex :type Integer) (bFromSweep :type Boolean) (SweepResult :type "HitResult Structure (by ref)"))
  (bind (_returnvalue_roll _returnvalue_pitch _returnvalue_yaw) (`KismetMathLibrary.BreakRotator` (`SceneComponent.K2_GetComponentRotation` (`self.Door`))))
  (bind (_returnvalue_roll_2 _returnvalue_pitch_2 _returnvalue_yaw_2) (`KismetMathLibrary.BreakRotator` (`SceneComponent.K2_GetComponentRotation` (`self.DoorFrame`))))
  (cast `/Game/FirstPerson/Blueprints/BP_FirstPersonCharacter` OtherActor)
  (if (< (`KismetMathLibrary.Abs` (+ (* _returnvalue_yaw -1.0) _returnvalue_yaw_2)) 5.0)
    (bind (_direction _doorswing) (`Timeline|Timeline` :!via `PlayFromStart`)
      (:`Update`
        (`SceneComponent.K2_SetRelativeRotation` (`self.Door`) (`KismetMathLibrary.MakeRotator` 0.0 0.0 (* (`KismetMathLibrary.Lerp` 0.0 120.0 _doorswing) -1.0)) false false)))))

(fn `UserConstructionScript`)