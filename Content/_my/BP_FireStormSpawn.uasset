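; BP_FireStormSpawn is a placed spawner that attacks a nearby player with a fire storm.
; A looping timer, with its interval randomized once at BeginPlay, checks whether the player pawn is within range.
; If so, it plays a small explosion at its Arrow, waits briefly, then spawns BP_FireStorm at the player's location.
; A Timeline scales the storm's particle system up from zero and destroys the storm when finished.
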(event `self.ReceiveBeginPlay`
  (`KismetSystemLibrary.K2_SetTimerDelegate` (delegate `spawnstorm`) (`KismetMathLibrary.RandomFloatInRange` 5.0 10.0) true))

(event `spawnstorm`
  (bind _output_get (set `self.PlayerPawnLocation` (`self.K2_GetActorLocation` (`GameplayStatics.GetPlayerPawn` 0))))
  (if (< (`KismetMathLibrary.Vector_Distance` _output_get (`self.K2_GetActorLocation`)) 1000.0)
    (`GameplayStatics.SpawnEmitterAtLocation` "/Game/FXVarietyPack/Particles/P_ky_explosion.P_ky_explosion" (`SceneComponent.K2_GetComponentLocation` (`self.Arrow`)) (struct) (0.05 0.05 0.05))
    (`KismetSystemLibrary.Delay` 1.0)
    (bind _returnvalue (`|SpawnActorFromClass` "/Game/_my/BP_FireStorm.BP_FireStorm_C" (`KismetMathLibrary.MakeTransform` (`self.PlayerPawnLocation`) (struct) (0.0 0.0 0.0)) "Undefined" "MultiplyWithRoot" null null))
    (bind (_direction _stormscale) (`Timeline|Timeline` :!via `PlayFromStart`)
      (:`Update`
        (bind _returnvalue_2 (`KismetMathLibrary.Lerp` 0.0 0.7 _stormscale))
        (`SceneComponent.SetWorldScale3D` (`/Game/_my/BP_FireStorm.ParticleSystem` _returnvalue) (`KismetMathLibrary.MakeVector` _returnvalue_2 _returnvalue_2 _returnvalue_2)))
      (:`Finished`
        (`self.K2_DestroyActor` _returnvalue)))))

(fn `UserConstructionScript`)