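; BP_CubeMove is a moving actor that can be temporarily frozen in place.
; On BeginPlay it runs the parent logic, caches its location, and sets an end point 900 units along world Y.
; A Timeline track named 010 drives a vector lerp between both points, moving the actor without sweeping.
; EventFreeze stops the Timeline, then resumes it from that position after FreezeDuration.
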(event `self.ReceiveBeginPlay`
  (`parent.ReceiveBeginPlay`)
  (bind _output_get (set `self.start position` (`self.K2_GetActorLocation`)))
  (set `self.end position` (+ _output_get (0.0 900.0 0.0)))
  (bind (_direction _0_1_0) (`Timeline|Timeline`)
    (:`Update`
      (`self.K2_SetActorLocation` (`KismetMathLibrary.VLerp` (`self.start position`) (`self.end position`) _0_1_0)))))

(event `self.Event Freeze`
  (`TimelineComponent.Stop` (`self.Timeline`))
  (`KismetSystemLibrary.Delay` (`self.Freeze duration`))
  (`TimelineComponent.Play` (`self.Timeline`)))

(fn `UserConstructionScript`
  (`parent.UserConstructionScript`))