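; BP_FireSpawn2 is a fire projectile emitter that shoots while activated and the player pawn is within 1000 units.
; A looping timer, with its interval randomized once at BeginPlay, spawns BP_FireProjectile at the Arrow's transform.
; The normalized direction to the player, scaled by a random speed, is applied as local-space velocity despite being a world-space vector.
; EventFreeze flips IsActivated, then flips it back after FreezeDuration.
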(event `self.Event Freeze`
  (set `self.IsActivated` (not (`self.IsActivated`)))
  (`KismetSystemLibrary.Delay` (`self.Freeze Duration`))
  (set `self.IsActivated` (not (`self.IsActivated`))))

(event `self.ReceiveBeginPlay`
  (`KismetSystemLibrary.K2_SetTimerDelegate` (delegate `spawnfireprojectile`) (`KismetMathLibrary.RandomFloatInRange` 0.7 1.5) true))

(event `spawnfireprojectile`
  (bind _arrow (`self.Arrow`))
  (if (`self.IsActivated`)
    (if (< (`KismetMathLibrary.Vector_Distance` (`self.K2_GetActorLocation` (`GameplayStatics.GetPlayerPawn` 0)) (`self.K2_GetActorLocation`)) 1000.0)
      (bind _returnvalue (`|SpawnActorFromClass` "/Game/_my/BP_FireProjectile.BP_FireProjectile_C" (`KismetMathLibrary.MakeTransform` (`SceneComponent.K2_GetComponentLocation` _arrow) (`SceneComponent.K2_GetComponentRotation` _arrow)) "Undefined" "MultiplyWithRoot" null null))
      (`ProjectileMovementComponent.SetVelocityInLocalSpace` (`/Game/_my/BP_FireProjectile.ProjectileMovement` _returnvalue) (* (`KismetMathLibrary.Normal` (- (`self.K2_GetActorLocation` (`GameplayStatics.GetPlayerPawn` 0)) (`self.K2_GetActorLocation`))) (`KismetMathLibrary.RandomFloatInRange` 1500.0 2000.0))))))

(fn `UserConstructionScript`
  (`parent.UserConstructionScript`))