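; Explosive barrel, a child of a destructible parent Blueprint, that blows up and kills nearby characters when destroyed.
; Its HandleDestroy override calls the parent, spawns scaled-up explosion and smoke emitters at the Destructible component, and fires a RadialForce impulse.
; It enables query collision on KillZone only at that moment, then deals massive environmental damage to every overlapping BP_Character.
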(fn `HandleDestroy`
  (params (NewParam :type "Vector Structure") (NewParam1 :type "HitResult Structure"))
  (bind _returnvalue (`SceneComponent.K2_GetComponentLocation` (`self.Destructible`)))
  (`parent.HandleDestroy` NewParam NewParam1)
  (`GameplayStatics.SpawnEmitterAtLocation` "/Game/StarterContent/Particles/P_Explosion.P_Explosion" _returnvalue (struct) (4.0 4.0 4.0))
  (`GameplayStatics.SpawnEmitterAtLocation` "/Game/StarterContent/Particles/P_Smoke.P_Smoke" _returnvalue (struct) (4.0 4.0 4.0))
  (`PrimitiveComponent.SetCollisionEnabled` (`self.KillZone`) "QueryOnly")
  (`RadialForceComponent.FireImpulse` (`self.RadialForce`))
  (for _array_element (`PrimitiveComponent.GetOverlappingActors` (`self.KillZone`) "/Game/Classes/BP_Character.BP_Character_C")
    (`GameplayStatics.ApplyDamage` _array_element 1000000.0 null null "/Engine/EngineDamageTypes/DmgTypeBP_Environmental.DmgTypeBP_Environmental_C")))

(fn `UserConstructionScript`
  (`parent.UserConstructionScript`))