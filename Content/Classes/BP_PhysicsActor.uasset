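; BP_PhysicsActor is a physics prop that can shatter into a Chaos destructible after hard impacts.
; Point damage flagged as world-caused pushes the simulating mesh along the hit normal, scaled by damage.
; While ungrabbed, hits at or above a speed threshold consume durability; a zero threshold disables destruction.
; Once durability is spent, the next hard hit swaps in the hidden Destructible, crumbles it with a radial impulse and plays a sound.
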(event `self.ReceivePointDamage`
  (params (Damage :type "Float (single-precision)") (DamageType :type "DamageType Object Reference") (HitLocation :type "Vector Structure") (HitNormal :type "Vector Structure") (HitComponent :type "PrimitiveComponent Object Reference") (BoneName :type Name) (ShotFromDirection :type "Vector Structure") (InstigatedBy :type "Controller Object Reference") (DamageCauser :type "Actor Object Reference") (HitInfo :type "HitResult Structure (by ref)"))
  (bind _physicsactorcomponent (`self.PhysicsActorComponent`))
  ;[0.04971 0.04971 0.04971] Handle Collision Force
  (if (and (`SceneComponent.IsSimulatingPhysics` _physicsactorcomponent "None") (`DamageType.bCausedByWorld` DamageType))
    (`PrimitiveComponent.AddVelocityChangeImpulseAtLocation` _physicsactorcomponent (* HitNormal Damage) HitLocation "None")))

(event `self.ReceiveHit`
  (params (MyComp :type "PrimitiveComponent Object Reference") (Other :type "Actor Object Reference") (OtherComp :type "PrimitiveComponent Object Reference") (bSelfMoved :type Boolean) (HitLocation :type "Vector Structure") (HitNormal :type "Vector Structure") (NormalImpulse :type "Vector Structure") (Hit :type "HitResult Structure (by ref)"))
  (bind _durability (`self.durability`))
  ;[0.04971 0.04971 0.04971] Handle Collision
  (`self.CanDestroy`
    (:`True`
      (if (not (`self.destroyed`))
        (bind _asbp_physics_actor_component (cast `/Game/Classes/BP_PhysicsActorComponent` MyComp))
        (if (`/Game/Classes/BP_PhysicsActorComponent.IsGrabbed` _asbp_physics_actor_component)
          _
          (elif (>= (`KismetMathLibrary.VSize` (`SceneComponent.GetComponentVelocity` (`self.PhysicsActorComponent`))) (`self.destructionThres`))
            (if (<= _durability 0)
              (`self.HandleDestroy` HitNormal Hit)
              (else
                (set `self.durability` (- _durability 1))))))))))

(fn `ChaosDestroy`
  (returns (ReturnValue :type "Vector Structure"))
  (bind _destructible (`self.Destructible`))
  (bind _static_mesh_component (`self.Static Mesh Component`))
  (`SceneComponent.SetVisibility` (`self.Static Mesh Component`) false false)
  (`SceneComponent.SetVisibility` _destructible true false)
  (`PrimitiveComponent.SetCollisionEnabled` _destructible "QueryAndPhysics")
  (`PrimitiveComponent.SetSimulatePhysics` _static_mesh_component false)
  (`PrimitiveComponent.SetCollisionEnabled` _static_mesh_component "NoCollision")
  (`GeometryCollectionComponent.CrumbleActiveClusters` (`self.Destructible`))
  (`PrimitiveComponent.AddRadialImpulse` (`self.Destructible`) (0.0 0.0 0.0) 1000.0 100.0 "RIF_Constant" true)
  (return (`SceneComponent.K2_GetComponentLocation` (`self.Destructible`))))

(fn `HandleDestroy`
  (params (NewParam :type "Vector Structure") (NewParam1 :type "HitResult Structure"))
  (bind _returnvalue (`self.ChaosDestroy`))
  (`GameplayStatics.PlaySoundAtLocation` (`self.destructionSound`) _returnvalue (struct) 1.0 1.0 0.0 null null null null)
  (set `self.destroyed` true))

(fn `UserConstructionScript`
  (bind _destructible (`self.Destructible`))
  (set `self.Static Mesh Component` (`self.PhysicsActorComponent`))
  (`SceneComponent.SetVisibility` _destructible false false)
  (`PrimitiveComponent.SetCollisionEnabled` _destructible "NoCollision"))