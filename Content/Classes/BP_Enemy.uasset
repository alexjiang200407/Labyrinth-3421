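; Enemy character that chases the player on sight and ragdolls when damaged or pushed by the gravity gun.
; While ragdolled, a downward trace from the pelvis keeps the capsule under the body.
; A looping timer triggers get-up once pelvis spin settles, unless heavy damage has killed it.
; Get-up orients the capsule to the lying pose and saves a pose snapshot, presumably for animation blending.
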(event `self.ReceiveBeginPlay`
  (set `self.pelvisOffset` (`SceneComponent.RelativeLocation` (`self.Mesh`))))

(event `self.PawnSensing.OnSeePawn`
  (params (Pawn :type "Pawn Object Reference"))
  (`self.FollowPawn`))

(event `FollowPawn`
  (`|AIMoveTo` self (0.0 0.0 0.0) (`GameplayStatics.GetPlayerCharacter` 0)))

(event `self.ReceiveAnyDamage`
  (params (Damage :type "Float (single-precision)") (DamageType :type "DamageType Object Reference") (InstigatedBy :type "Controller Object Reference") (DamageCauser :type "Actor Object Reference"))
  (if (not (`self.ragdolling`))
    (`self.Ragdoll` (0.0 0.0 0.0))
    (if (>= Damage 5000.0)
      (set `self.dead` true))))

(event `self.ReceiveTick`
  (params (DeltaSeconds :type "Float (single-precision)"))
  (if (`self.ragdolling`)
    (`self.UpdateCapsuleLocation`)))

(event `GetUpFromRagdoll`
  (bind _mesh (`self.Mesh`))
  (if (`self.ragdolling`)
    (`self.FindCharacterOrientation`)
    (`self.SetCapsuleOrientation`)
    (`KismetSystemLibrary.Delay` 0.0)
    (`KismetSystemLibrary.Delay` 0.0)
    (`AnimInstance.SavePoseSnapshot` (`SkeletalMeshComponent.GetAnimInstance` (`self.Mesh`)) "RagdollFinalPose")
    (`KismetSystemLibrary.Delay` 0.0)
    (set `self.ragdolling` false)
    (`PrimitiveComponent.SetSimulatePhysics` _mesh false)
    (`PrimitiveComponent.SetCollisionEnabled` _mesh "NoCollision")
    (`PrimitiveComponent.SetCollisionEnabled` (`self.CapsuleComponent`) "QueryAndPhysics")))

(event `ToAnimationFinal`
  (`CharacterMovementComponent.SetMovementMode` (`self.CharacterMovement`) "MOVE_Walking" 0)
  (set `self.DoIK` true))

(event `/Game/Classes/BP_Pushable.GravityGunPush`
  (params (Impulse :type "Vector Structure"))
  (`self.Ragdoll` Impulse))

(fn `FindCharacterOrientation`
  (bind (_returnvalue_x _returnvalue_y _returnvalue_z) (`KismetMathLibrary.BreakVector` (`KismetMathLibrary.GetRightVector` (`SceneComponent.GetSocketRotation` (`self.Mesh`) "pelvis"))))
  (set `self.layingOnBack` (> _returnvalue_z 0.0)))

(fn `Ragdoll`
  (params (Impulse :type "Vector Structure"))
  (bind _mesh (`self.Mesh`))
  (if (not (`self.ragdolling`))
    (set `self.ragdolling` true)
    (set `self.DoIK` false)
    (`PrimitiveComponent.SetCollisionEnabled` _mesh "QueryAndPhysics")
    (`PrimitiveComponent.SetSimulatePhysics` _mesh true)
    (`SkeletalMeshComponent.AddImpulseToAllBodiesBelow` _mesh Impulse "pelvis" true true)
    (`CharacterMovementComponent.SetMovementMode` (`self.CharacterMovement`) "MOVE_None" 0)
    (`PrimitiveComponent.SetCollisionEnabled` (`self.CapsuleComponent`) "QueryOnly")
    (`KismetSystemLibrary.K2_SetTimer` null "ShouldEndRagdoll" 0.2 true true)))

(fn `SetCapsuleOrientation`
  (bind _mesh (`self.Mesh`))
  (bind _returnvalue (- (`SceneComponent.GetSocketLocation` _mesh "neck_01") (`SceneComponent.GetSocketLocation` _mesh "pelvis")))
  (`SceneComponent.K2_SetWorldRotation` (`self.CapsuleComponent`) (`KismetMathLibrary.MakeRotFromZX` (`KismetMathLibrary.MakeVector` 0.0 0.0 1.0) (`KismetMathLibrary.SelectVector` (* _returnvalue -1.0) _returnvalue (`self.layingOnBack`))) false false))

(fn `ShouldEndRagdoll`
  (if (or (`self.dead`) (not (`self.ragdolling`)))
    (`KismetSystemLibrary.K2_ClearTimer` null "ShouldEndRagdoll" :!label _label)
    (elif (<= (`KismetMathLibrary.VSize` (`PrimitiveComponent.GetPhysicsAngularVelocityInDegrees` (`self.Mesh`) "pelvis")) 10.0)
      (`self.GetUpFromRagdoll`)
      (goto _label))))

(fn `UpdateCapsuleLocation`
  (bind _returnvalue (`SceneComponent.GetSocketLocation` (`self.Mesh`) "pelvis"))
  (bind (_outhit _returnvalue_2) (`KismetSystemLibrary.LineTraceSingle` _returnvalue (+ _returnvalue (0.0 0.0 -100.0)) "TraceTypeQuery1"))
  (if _returnvalue_2
    (set `self.targetGroundLocation` (`.Location` (`GameplayStatics.BreakHitResult` _outhit)))
    (else
      (set `self.targetGroundLocation` _returnvalue)))
  (bind _output_get (set `self.meshLocation` (- (`self.targetGroundLocation`) (`self.pelvisOffset`))))
  (`SceneComponent.K2_SetWorldLocation` (`self.CapsuleComponent`) _output_get false false))

(fn `UserConstructionScript`)